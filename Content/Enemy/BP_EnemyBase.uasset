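; Base enemy Blueprint for flipbook-sprite enemies that turns to match horizontal movement and passes its type enum to the AI blackboard.
; Health, healing and damage calls forward to BPCDamageSystem, with a health bar widget bound to the enemy.
; The component's death event switches on type: most destroy after a short delay, while Explode damages one sphere-trace hit and plays an explosion flipbook before destruction.
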(event `self.ReceiveTick`
  (params (DeltaSeconds :type "Float (single-precision)"))
  (bind _returnvalue_x (`KismetMathLibrary.BreakVector` (`self.GetVelocity`)))
  (`/Engine/EditorBlueprintResources/StandardMacros.CompareFloat` (* DeltaSeconds _returnvalue_x)
    (:`>`
      (`self.K2_SetActorRotation` (struct)))
    (:`<`
      (`self.K2_SetActorRotation` (struct :`Yaw` 180.0)))))

(event `self.ReceiveBeginPlay`
  (`|ExecutionSequence`
    (:`then_0`
      (`BlackboardComponent.SetValueAsEnum` (`AIBlueprintHelperLibrary.GetBlackboard` null) "EnemyType" (`self.EnemyEnum`)))
    (:`then_1`
      (bind _returnvalue (`|CreateWidget` "/Game/Widgets/W_HealthBar.W_HealthBar_C" null self))
      (`WidgetComponent.SetWidget` (`self.Widget`) _returnvalue))))

(event `Death`
  (bind _returnvalue (`self.K2_GetActorLocation`))
  (switch `/Game/Enemy/EEnemyType` (`self.EnemyEnum`)
    (:`NewEnumerator0`
      ;[1 1 1] Testing
      (`KismetSystemLibrary.PrintString` "EnemyDead" :!label _label)
      (`KismetSystemLibrary.Delay` 0.5)
      (`self.K2_DestroyActor`))
    (:`NewEnumerator1`
      (goto _label))
    (:`NewEnumerator2`
      (goto _label))
    (:`NewEnumerator3`
      (bind (_outhit _returnvalue_2) (`KismetSystemLibrary.SphereTraceSingleForObjects` :`Start` _returnvalue :`End` _returnvalue :`Radius` 200.0 :`ObjectTypes` (`|MakeArray` "ObjectTypeQuery8" "ObjectTypeQuery9" :!type "EObjectTypeQuery Enum") :`DrawDebugType` "ForDuration"))
      (if _returnvalue_2
        (message `/Game/Interfaces/BPI_Damagable.TakeDamage` (`.HitActor` (`GameplayStatics.BreakHitResult` _outhit)) (make `/Game/Interfaces/S_DamageInfo` 30.0 "NewEnumerator3"))
        (`self.ExplodingEnemyTimeFlipbookVfxSfx`)
        (else
          (`self.ExplodingEnemyTimeFlipbookVfxSfx`))))))

(fn `GetCurrentHealth`
  (returns (Health :type "Float (double-precision)"))
  (return (`/Game/Components/BPC_DamageSystem.Health` (`self.BPC_DamageSystem`))))

(fn `GetMaxHealth`
  (returns (MaxHealth :type "Float (double-precision)"))
  (return (`/Game/Components/BPC_DamageSystem.MaxHealth` (`self.BPC_DamageSystem`))))

(fn `Heal`
  (params (Amount :type "Float (double-precision)"))
  (returns (NewHealth :type "Float (double-precision)"))
  (bind _newhealth (`/Game/Components/BPC_DamageSystem.Heal` (`self.BPC_DamageSystem`) Amount))
  (return _newhealth))

(fn `TakeDamage`
  (params (DamageInfo :type "/Game/Interfaces/S_DamageInfo Structure"))
  (returns (WasDamaged :type Boolean))
  (bind _wasdamaged (`/Game/Components/BPC_DamageSystem.TakeDamage` (`self.BPC_DamageSystem`) DamageInfo))
  (return _wasdamaged))

(fn `UserConstructionScript`
  (add `/Game/Components/BPC_DamageSystem.OnDeath` (`self.BPC_DamageSystem`) (`|CreateDelegate` :!event `Death`)))