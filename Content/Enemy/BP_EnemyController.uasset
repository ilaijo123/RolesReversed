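; AI controller for enemies that runs the enemy behavior tree and keeps them targeting the nearest of the player support actor and the hero AI.
; On BeginPlay it caches one PlayerSupport and one BP_HeroAI (Witcher), then starts a looping half-second timer.
; Each tick of that timer finds whichever is closer to the controlled pawn and writes it to the TargetActor blackboard key.
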(event `self.ReceiveBeginPlay`
  (`|ExecutionSequence`
    (:`then_0`
      (bind _returnvalue (`GameplayStatics.GetActorOfClass` "/Game/Characters/SupportCharacter/PlayerSupport.PlayerSupport_C"))
      (`/Engine/EditorBlueprintResources/StandardMacros.IsValid` _returnvalue
        (:`Is Valid`
          (set `self.Player` _returnvalue))))
    (:`then_1`
      (bind _returnvalue_2 (`GameplayStatics.GetActorOfClass` "/Game/Characters/HeroAI/BP_HeroAI.BP_HeroAI_C"))
      (`/Engine/EditorBlueprintResources/StandardMacros.IsValid` _returnvalue_2
        (:`Is Valid`
          (set `self.Witcher` _returnvalue_2))))
    (:`then_3`
      (`KismetSystemLibrary.K2_SetTimerDelegate` (delegate `RefreshTarget`) 0.5 true))))

(event `RefreshTarget`
  (bind _returnvalue (`self.GetClosestTarget`))
  (`/Engine/EditorBlueprintResources/StandardMacros.IsValid` _returnvalue
    (:`Is Valid`
      (`BlackboardComponent.SetValueAsObject` (`self.Blackboard`) "TargetActor" _returnvalue))))

(event `self.ReceivePossess`
  (params (PossessedPawn :type "Pawn Object Reference"))
  (`self.RunBehaviorTree` "/Game/Enemy/BT_EnemyBehaviour.BT_EnemyBehaviour"))

(fn `GetClosestTarget`
  (returns (ReturnValue :type "Actor Object Reference"))
  (return (`.ReturnValue` (`GameplayStatics.FindNearestActor` (`self.K2_GetActorLocation` (`self.K2_GetPawn`)) (`|MakeArray` (`self.Witcher`) (`self.Player`) :!type "Actor Object Reference")))))

(fn `UserConstructionScript`)