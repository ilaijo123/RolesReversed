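; Enemy spawner actor that periodically spawns a random melee, exploding or projectile enemy at a reachable point around itself.
; A looping timer picks a random navigable location within a random radius between the min and max bounds, then moves a Paper2D flipbook there to play a spawn effect as a telegraph.
; A delayed follow-up timer clears the effect and spawns the enemy at that stored location.
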(event `self.ReceiveBeginPlay`
  (`KismetSystemLibrary.K2_SetTimerDelegate` (delegate `GetRandomPoint`) (`KismetMathLibrary.RandomFloatInRange` 6.0 6.0) true))

(event `GetRandomPoint`
  (set `self.RandomLocation` (`NavigationSystemV1.K2_GetRandomReachablePointInRadius` (`self.K2_GetActorLocation`) (`KismetMathLibrary.RandomFloatInRange` (`self.MinRadius`) (`self.MaxRadius`)) null null))
  (`SceneComponent.K2_SetWorldLocation` (`self.PaperFlipbook`) (`self.RandomLocation`) false false)
  (`PaperFlipbookComponent.SetFlipbook` (`self.PaperFlipbook`) (`self.SpawnEffect`))
  (`KismetSystemLibrary.K2_SetTimerDelegate` (delegate `SpawnEnemy`) 3.0))

(event `SpawnEnemy`
  (`PaperFlipbookComponent.SetFlipbook` (`self.PaperFlipbook`) null)
  (`|SpawnActorFromClass` (`KismetArrayLibrary.Array_Random` (`|MakeArray` (`self.MeleeEnemy`) (`self.ExplodingEnemy`) (`self.ProjectileEnemy`) :!type "Actor Class Reference")) (`KismetMathLibrary.MakeTransform` (`self.RandomLocation`)) "Undefined" "MultiplyWithRoot" null null))

(fn `UserConstructionScript`)